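; A platform button actor that the third-person character can press with E while overlapping it, apparently meant to control a linked moving platform.
; Tick finds and caches the player character, while actor overlap events set the Overlapping flag and both enable input for its controller.
; Pressing E casts the linked Platform to movingplatform and stores it, then checks ButtonOnPlatform and Top, but those branches perform no action.
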(event `self.ReceiveTick`
  (params (DeltaSeconds :type "Float (single-precision)"))
  (`/Engine/EditorBlueprintResources/StandardMacros.IsValid` (`self.player`)
    (:`Is Not Valid`
      (bind _returnvalue (`GameplayStatics.GetActorOfClass` "/Game/ThirdPerson/Blueprints/BP_ThirdPersonCharacter.BP_ThirdPersonCharacter_C"))
      (set `self.player` _returnvalue))))

(event `OnComponentBeginOverlap_Event`
  (params (OverlappedComponent :type "PrimitiveComponent Object Reference") (OtherActor :type "Actor Object Reference") (OtherComp :type "PrimitiveComponent Object Reference") (OtherBodyIndex :type Integer) (bFromSweep :type Boolean) (SweepResult :type "HitResult Structure (by ref)")))

(event `self.ReceiveActorBeginOverlap`
  (params (OtherActor :type "Actor Object Reference"))
  (cast `/Game/ThirdPerson/Blueprints/BP_ThirdPersonCharacter` OtherActor)
  (set `self.Overlapping` true)
  (`self.EnableInput` (`PlayerState.GetPlayerController` (`Pawn.PlayerState` (`self.player`)))))

(event `OnComponentEndOverlap_Event`
  (params (OverlappedComponent :type "PrimitiveComponent Object Reference") (OtherActor :type "Actor Object Reference") (OtherComp :type "PrimitiveComponent Object Reference") (OtherBodyIndex :type Integer)))

(event `self.ReceiveActorEndOverlap`
  (params (OtherActor :type "Actor Object Reference"))
  (cast `/Game/ThirdPerson/Blueprints/BP_ThirdPersonCharacter` OtherActor)
  (set `self.Overlapping` false)
  (`self.EnableInput` (`PlayerState.GetPlayerController` (`Pawn.PlayerState` (`self.player`)))))

(event `Key|E`
  (params (Key :type "Key Structure"))
  (bind _platform (`self.Platform`))
  (:`Pressed`
    (if (`self.Overlapping`)
      (`/Engine/EditorBlueprintResources/StandardMacros.IsValid` _platform
        (:`Is Valid`
          (bind _asmovingplatform (cast `/Game/Blueprints/movingplatform` _platform))
          (set `self.PlatformRef` _asmovingplatform)
          (if (`self.ButtonOnPlatform`)
            _
            (elif (`self.Top`)
              _)))))))

(fn `UserConstructionScript`)