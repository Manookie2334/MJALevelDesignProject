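; ButtonBP is an interactable button that toggles a referenced DoorBP open and closed when E is pressed.
; Overlap handlers for BP_ThirdPersonCharacter set an Overlapping flag and enable or disable input through the Player reference's controller.
; While overlapping, E casts the Door reference and a FlipFlop alternates OpenDoor and CloseDoor.
; The nodes that bind both overlap handlers are never executed in this graph.
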(event `OnComponentBeginOverlap_Event`
  (params (OverlappedComponent :type "PrimitiveComponent Object Reference") (OtherActor :type "Actor Object Reference") (OtherComp :type "PrimitiveComponent Object Reference") (OtherBodyIndex :type Integer) (bFromSweep :type Boolean) (SweepResult :type "HitResult Structure (by ref)"))
  (cast `/Game/ThirdPerson/Blueprints/BP_ThirdPersonCharacter` OtherActor)
  (set `self.overlapping` true)
  (`self.EnableInput` (`PlayerState.GetPlayerController` (`Pawn.PlayerState` (`self.player`)))))

(event `OnComponentEndOverlap_Event`
  (params (OverlappedComponent :type "PrimitiveComponent Object Reference") (OtherActor :type "Actor Object Reference") (OtherComp :type "PrimitiveComponent Object Reference") (OtherBodyIndex :type Integer))
  (cast `/Game/ThirdPerson/Blueprints/BP_ThirdPersonCharacter` OtherActor)
  (set `self.overlapping` false)
  (`self.DisableInput` (`PlayerState.GetPlayerController` (`Pawn.PlayerState` (`self.player`)))))

(event `Key|E`
  (params (Key :type "Key Structure"))
  (bind _casteddoor (`self.CastedDoor`))
  (:`Pressed`
    (if (`self.overlapping`)
      (`/Engine/EditorBlueprintResources/StandardMacros.IsValid` (`self.Door`)
        (:`Is Valid`
          (bind _asdoor_bp (cast `/Game/Blueprints/DoorBP` (`self.Door`)))
          (set `self.CastedDoor` _asdoor_bp)
          (`/Engine/EditorBlueprintResources/StandardMacros.FlipFlop`
            (:`A`
              (`/Game/Blueprints/DoorBP.open door` _casteddoor))
            (:`B`
              (`/Game/Blueprints/DoorBP.close door` _casteddoor))))))))

(fn `UserConstructionScript`)