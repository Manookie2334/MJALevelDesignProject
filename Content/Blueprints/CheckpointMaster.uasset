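; CheckpointMaster is a checkpoint manager actor that stores a respawn location and returns the player to it.
; On Tick it looks up the BP_ThirdPersonCharacter whenever its player reference is invalid.
; A setRespawnPoint event updates the saved position, and a Respawn event teleports the player there without sweeping.
; Ragdoll physics toggles and a timeline-delayed respawn remain in the graph, but no event triggers them.
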(event `self.ReceiveTick`
  (params (DeltaSeconds :type "Float (single-precision)"))
  (`/Engine/EditorBlueprintResources/StandardMacros.IsValid` (`self.player`)
    (:`Is Not Valid`
      (bind _returnvalue (`GameplayStatics.GetActorOfClass` "/Game/ThirdPerson/Blueprints/BP_ThirdPersonCharacter.BP_ThirdPersonCharacter_C"))
      (set `self.player` _returnvalue))))

(event `setRespawnPoint`
  (params (POS :type "Vector Structure"))
  (set `self.pointPOS` POS))

(event `Respawn`
  (`self.K2_SetActorLocation` (`self.Player`) (`self.pointPOS`) false false))

(fn `UserConstructionScript`)