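; Actor Blueprint that moves itself back and forth between its starting location and an EndPOS world position.
; On BeginPlay it stores the start location, then a Timeline alpha drives a location lerp without sweep.
; When the Timeline finishes, the StartEnd flag toggles and selects reverse or forward playback, so the motion loops indefinitely.
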(event `self.ReceiveBeginPlay`
  (set `self.startPOS` (`self.K2_GetActorLocation`))
  (bind (_direction _alp) (`Timeline|Timeline` :!via `PlayFromStart` :!label _label)
    (:`Update`
      (`self.K2_SetActorLocation` (`KismetMathLibrary.VLerp` (`self.startPOS`) (`self.endPOS`) _alp)))
    (:`Finished`
      (if (`self.StartEnd`)
        (set `self.StartEnd` false)
        (goto _label :!via `PlayFromStart`)
        (else
          (set `self.StartEnd` true)
          (goto _label :!via `ReverseFromEnd`))))))

(fn `UserConstructionScript`)