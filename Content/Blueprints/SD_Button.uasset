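; SD_Button is an interactable button that sets a CountdownTrigger flag when the player presses E within its overlap area.
; Tick looks up the BP_ThirdPersonCharacter until the Player reference is valid.
; Begin and end overlap with that character class set the Overlapping flag and enable or disable input for the cached player's controller.
; The flag is only set true here, with no reset or countdown logic.
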(event `self.ReceiveTick`
  (params (DeltaSeconds :type "Float (single-precision)"))
  (`/Engine/EditorBlueprintResources/StandardMacros.IsValid` (`self.player`)
    (:`Is Not Valid`
      (bind _returnvalue (`GameplayStatics.GetActorOfClass` "/Game/ThirdPerson/Blueprints/BP_ThirdPersonCharacter.BP_ThirdPersonCharacter_C"))
      (set `self.player` _returnvalue))))

(event `self.ReceiveActorBeginOverlap`
  (params (OtherActor :type "Actor Object Reference"))
  (cast `/Game/ThirdPerson/Blueprints/BP_ThirdPersonCharacter` OtherActor)
  (set `self.overlapping` true)
  (`self.EnableInput` (`PlayerState.GetPlayerController` (`Pawn.PlayerState` (`self.player`)))))

(event `self.ReceiveActorEndOverlap`
  (params (OtherActor :type "Actor Object Reference"))
  (cast `/Game/ThirdPerson/Blueprints/BP_ThirdPersonCharacter` OtherActor)
  (set `self.overlapping` false)
  (`self.DisableInput` (`PlayerState.GetPlayerController` (`Pawn.PlayerState` (`self.player`)))))

(event `Key|E`
  (params (Key :type "Key Structure"))
  (:`Pressed`
    (if (`self.overlapping`)
      (set `self.CountdownTrigger` true))))

(fn `UserConstructionScript`)